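; BP_Arquero is an archer actor that periodically shoots arrows.
; BeginPlay starts a looping timer on TiempoDisparo that spawns a BP_Flecha at the actor's transform whenever the Dispara flag is on.
; Each arrow's speed is VelocidadFlecha multiplied by Factor.
; Setter functions let the arrow speed and the firing flag be changed.
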(event Custom|Disparar
  (if (Variables|Propiedades|GetbDispara)
    (CallFunction|SpawnearFlecha)))

(event EventBeginPlay
  (Utilities|Time|SetTimerbyEvent (delegate Custom|Disparar) (Variables|Propiedades|GetTiempoDisparo) true))

(event Collision|EventActorBeginOverlap
  (params (OtherActor :type Actor%20Object%20Reference)))

(event EventTick
  (params (DeltaSeconds :type Float%20%28single-precision%29)))

(fn ConstructionScript)

(fn SpawnearFlecha
  (Game|SpawnActorfromClass "/Game/Blueprints/BP_Flecha.BP_Flecha_C" (Transformation|GetActorTransform) "Undefined" "MultiplyWithRoot" 0 (* (Variables|Propiedades|GetVelocidadFlecha) (Variables|Propiedades|GetFactor)) 0))

(fn SetearVelocidadFlecha
  (params (VelocidadFlecha :type Vector))
  (Variables|Propiedades|SetVelocidadFlecha VelocidadFlecha))

(fn SetearDispara
  (params (bDispara :type Boolean))
  (Variables|Propiedades|SetbDispara bDispara))